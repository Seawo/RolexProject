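; BP_Character_Phase is the Phase character Blueprint, with keyboard shortcuts that trigger its animations, apparently for preview or testing.
; The P, O, I and U keys each play a montage on the Mesh: death, victory, start and stun respectively, with death starting at its Die1 section.
; The event graph holds no other logic, and the construction script is empty.
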(event Input|KeyboardEvents|U
  (params (Key :type Key%20Structure :default "None"))
  (:Pressed
    (Animation|Montage|PlayMontage (Variables|Character|GetMesh) "/Game/Rolex/LSH/Blueprints/Phase/Animation/AM_Phase_Stun.AM_Phase_Stun" 1.0 0.0 "")))

(event Input|KeyboardEvents|P
  (params (Key :type Key%20Structure :default "None"))
  (:Pressed
    (Animation|Montage|PlayMontage (Variables|Character|GetMesh) "/Game/Rolex/LSH/Blueprints/Phase/Animation/AM_Phase_Die.AM_Phase_Die" 1.0 0.0 "Die1")))

(event Input|KeyboardEvents|O
  (params (Key :type Key%20Structure :default "None"))
  (:Pressed
    (Animation|Montage|PlayMontage (Variables|Character|GetMesh) "/Game/Rolex/LSH/Blueprints/Phase/Animation/AM_Phase_Victory.AM_Phase_Victory" 1.0 0.0 "")))

(event Input|KeyboardEvents|I
  (params (Key :type Key%20Structure :default "None"))
  (:Pressed
    (Animation|Montage|PlayMontage (Variables|Character|GetMesh) "/Game/Rolex/LSH/Blueprints/Phase/Animation/AM_Phase_Start.AM_Phase_Start" 1.0 0.0 "")))

(fn ConstructionScript)